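; BP_TimeBomb is an area-effect actor that slows time for the player character and AI guards overlapping it.
; A two-second delay after BeginPlay arms it by setting CanTakeAffect, then flows into the same slow branch used by BeginOverlap.
; Once armed, overlap begin and end set each ThirdPersonCharacter or AI_Guard's CustomTimeDilation to slow or normal, leaving global time untouched.
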(event Collision|EventActorEndOverlap
  (params (OtherActor :type Actor%20Object%20Reference))
  (bind _normaldilation (Variables|Default|GetNormalDilation))
  ;[1 1 1] On EndOverlap, Restore Time Dilation
  (if (Variables|Default|GetCanTakeAffect?)
    (bind _asthird_person_character (Utilities|Casting|CastToThirdPersonCharacter OtherActor)
      (:then
        (Variables|/Script/Engine.Actor|SetCustomTimeDilation _asthird_person_character _normaldilation))
      (:CastFailed
        (bind _asai_guard (Utilities|Casting|CastToAI_Guard OtherActor))
        (Variables|/Script/Engine.Actor|SetCustomTimeDilation _asai_guard _normaldilation)))))

(event Collision|EventActorBeginOverlap
  (params (OtherActor :type Actor%20Object%20Reference))
  (bind _slowdilation (Variables|Default|GetSlowDilation))
  ;[1 1 1] On BeginOverlap, Slow Time Dilation
  (if (Variables|Default|GetCanTakeAffect?)
    (bind _asthird_person_character (Utilities|Casting|CastToThirdPersonCharacter OtherActor)
      (:then
        (Variables|/Script/Engine.Actor|SetCustomTimeDilation _asthird_person_character _slowdilation))
      (:CastFailed
        (bind _asai_guard (Utilities|Casting|CastToAI_Guard OtherActor))
        (Variables|/Script/Engine.Actor|SetCustomTimeDilation _asai_guard _slowdilation)))))

(event EventBeginPlay
  (bind _slowdilation (Variables|Default|GetSlowDilation))
  ;[1 1 1] On Spawn, Begin Countdown
  (Utilities|FlowControl|DoOnce false
    (:Completed
      (Utilities|FlowControl|Delay 2.0)
      (Variables|Default|SetCanTakeAffect? true)
      ;[1 1 1] On BeginOverlap, Slow Time Dilation
      (bind _asthird_person_character (Utilities|Casting|CastToThirdPersonCharacter (stale Collision|EventActorBeginOverlap OtherActor))
        (:then
          (Variables|/Script/Engine.Actor|SetCustomTimeDilation _asthird_person_character _slowdilation))
        (:CastFailed
          (bind _asai_guard (Utilities|Casting|CastToAI_Guard (stale Collision|EventActorBeginOverlap OtherActor)))
          (Variables|/Script/Engine.Actor|SetCustomTimeDilation _asai_guard _slowdilation))))))

(fn ConstructionScript)