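; Interactable door actor that swings open and closed when RotateDoor is triggered while the player is inside its box.
; Box overlap events set PlayerOverlapped for ThirdPersonCharacter only.
; RotateDoor uses a FlipFlop to play or reverse the DoorRotation timeline, which drives the door's relative yaw.
; An older timer-based poll of the player's InteractActor through CheckIfPlayerInteract remains but is disconnected, and nothing in this Blueprint starts it.
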(event OnComponentBeginOverlap(Box)
  (params (OverlappedComponent :type Primitive%20Component%20Object%20Reference) (OtherActor :type Actor%20Object%20Reference) (OtherComp :type Primitive%20Component%20Object%20Reference) (OtherBodyIndex :type Integer) (bFromSweep :type Boolean) (SweepResult :type Hit%20Result%20Structure%20%28by%20ref%29))
  ;[1 1 1] Set Variable Depending On If Player Overlapped
  (Utilities|Casting|CastToThirdPersonCharacter OtherActor) ; 3rdPersonChar will be primary char (temp?)
  (Variables|Default|SetPlayerOverlapped? true))

(event OnComponentEndOverlap(Box)
  (params (OverlappedComponent :type Primitive%20Component%20Object%20Reference) (OtherActor :type Actor%20Object%20Reference) (OtherComp :type Primitive%20Component%20Object%20Reference) (OtherBodyIndex :type Integer))
  ;[1 1 1] Set Variable Depending On If Player Overlapped
  (Utilities|Casting|CastToThirdPersonCharacter OtherActor) ; 3rdPersonChar will be primary char (temp?)
  (Variables|Default|SetPlayerOverlapped? false))

(event Custom|RotateDoor
  ;[1 1 1] If Player Interacts and If Player also Overlapped then open door
  (if (Variables|Default|GetPlayerOverlapped?)
    (Utilities|FlowControl|FlipFlop
      (:A
        (bind _doorrotation (Timeline|DoorRotation Play)
          (:Update
            (Transformation|SetRelativeRotation (Variables|Default|GetDoor) (Math|Rotator|MakeRotator 0.0 0.0 _doorrotation) false false))))
      (:B
        (Timeline|DoorRotation Reverse)))))

(fn ConstructionScript)

(fn CheckifPlayerInteract
  (bind _asthird_person_character (Utilities|Casting|CastToThirdPersonCharacter (Game|GetPlayerCharacter 0)))
  (if (== (Variables|/Game/ThirdPersonBP/ThirdPersonCharacter.ThirdPersonCharacter_C|GetInteractActor _asthird_person_character) self)
    (CallFunction|RotateDoor)))